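; Trigger actor that ends a Toon Tanks level when the player's tank overlaps it and moves play on to the next level.
; On overlap with BP_PawnTank it calls GameOver as a win on the game mode cached at BeginPlay.
; After a delay it shows the WBP_FadeOut widget, then briefly waits and opens the next level through a hardcoded switch on the current level name.
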(event EventBeginPlay
  (bind _asbp_toon_tanks_game_mode (Utilities|Casting|CastToBP_ToonTanksGameMode (Game|GetGameMode)))
  (Variables|Default|SetGameMode _asbp_toon_tanks_game_mode))

(event Collision|EventActorBeginOverlap
  (params (OtherActor :type Actor%20Object%20Reference))
  (Utilities|Casting|CastToBP_PawnTank OtherActor)
  (Class|ToonTanksGameMode|GameOver (Variables|Default|GetGameMode) true)
  (Utilities|FlowControl|Delay 4.0)
  (bind _returnvalue (UserInterface|CreateWidget "/Game/Blueprints/Widgets/Transitions/WBP_FadeOut.WBP_FadeOut_C"))
  (UserInterface|Viewport|AddtoViewport _returnvalue 0)
  (Utilities|FlowControl|Delay 0.5)
  (bind _returnvalue_2 (Game|GetCurrentLevelName true))
  (switch string _returnvalue_2
    (:Main
      (Game|OpenLevel(byName) "Level2"))
    (:Level2
      (Game|OpenLevel(byName) "Level3"))))

(event EventTick
  (params (DeltaSeconds :type Float%20%28single-precision%29)))

(fn ConstructionScript)