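; Game mode Blueprint for Toon Tanks that drives the match UI and level transitions through start, game-over and end-game events.
; StartGame shows start and score widgets, while GameOver shows win, level-complete or loss text, treating Level3 as the final level by name.
; A loss fades out and reloads the current level after delays; EndGame similarly fades to the main menu, and the win branch itself loads nothing.
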(event Custom|EndGame
  (Utilities|FlowControl|Delay 3.0)
  (CallFunction|FadeOut)
  (Utilities|FlowControl|Delay 0.5)
  (Game|OpenLevel(byName) "MainMenuLevel"))

(event Custom|FadeOut
  (bind _returnvalue (UserInterface|CreateWidget "/Game/Blueprints/Widgets/Transitions/WBP_FadeOut.WBP_FadeOut_C"))
  (UserInterface|Viewport|AddtoViewport _returnvalue 0))

(event EventBeginPlay)

(event EventTick
  (params (DeltaSeconds :type Float%20%28single-precision%29)))

(event EventStartGame
  (bind _returnvalue (UserInterface|CreateWidget "/Game/Blueprints/Widgets/HUD/WBP_StartGameWidget.WBP_StartGameWidget_C"))
  (UserInterface|Viewport|AddtoViewport _returnvalue 0)
  (bind _returnvalue_2 (UserInterface|CreateWidget "/Game/Blueprints/Widgets/HUD/WBP_ScoreWidget.WBP_ScoreWidget_C"))
  (UserInterface|Viewport|AddtoViewport _returnvalue_2 0))

(event EventGameOver
  (params (bWonGame :type Boolean))
  (bind _returnvalue (UserInterface|CreateWidget "/Game/Blueprints/Widgets/HUD/WBP_EndGameWidget.WBP_EndGameWidget_C"))
  (UserInterface|Viewport|AddtoViewport _returnvalue 0)
  (if bWonGame
    (bind _returnvalue_2 (Game|GetCurrentLevelName true))
    (if (Utilities|Enum|Equal(Enum) _returnvalue_2 "Level3")
      (Rendering|Components|TextRender|SetText (Variables|/Game/Blueprints/Widgets/HUD/WBP_EndGameWidget.WBP_EndGameWidget_C|GetDisplayText _returnvalue) "You Win!")
      (else
        (Rendering|Components|TextRender|SetText (Variables|/Game/Blueprints/Widgets/HUD/WBP_EndGameWidget.WBP_EndGameWidget_C|GetDisplayText _returnvalue) "Level Complete!")))
    (else
      (Rendering|Components|TextRender|SetText (Variables|/Game/Blueprints/Widgets/HUD/WBP_EndGameWidget.WBP_EndGameWidget_C|GetDisplayText _returnvalue) "You Lost!")
      (Utilities|FlowControl|Delay 3.0)
      (CallFunction|FadeOut)
      (Utilities|FlowControl|Delay 0.5)
      (bind _returnvalue_3 (Game|GetCurrentLevelName true))
      (Game|OpenLevel(byName) (Utilities|String|StringToName _returnvalue_3)))))

(fn ConstructionScript)